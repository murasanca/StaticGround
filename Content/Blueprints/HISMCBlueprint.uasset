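; Blueprint that turns the instances of its HierarchicalInstancedStaticMesh into a crowd of spawned Manny and Quinn characters at BeginPlay.
; Each instance spawns one of four random character variants at its local-space X/Y, with a fixed height, the same rotation and reduced scale.
; It then chains each variant class through Target, pointing every character at the previous one.
; The first of each chain targets itself and has actor tick disabled.
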(event `self.ReceiveBeginPlay`
  (bind _hierarchicalinstancedstaticmesh (`self.HierarchicalInstancedStaticMesh`))
  (for _index (range (`InstancedStaticMeshComponent.GetInstanceCount` _hierarchicalinstancedstaticmesh))
    (`|SpawnActorFromClass` (select `int` (`KismetMathLibrary.RandomInteger` 4) :`0` "/Game/Blueprints/CharacterBlueprintSKMManny.CharacterBlueprintSKMManny_C" :`1` "/Game/Blueprints/CharacterBlueprintSKMMannySimple.CharacterBlueprintSKMMannySimple_C" :`2` "/Game/Blueprints/CharacterBlueprintSKMQuinn.CharacterBlueprintSKMQuinn_C" :`3` "/Game/Blueprints/CharacterBlueprintSKMQuinnSimple.CharacterBlueprintSKMQuinnSimple_C" :!type "Actor Class Reference") (`KismetMathLibrary.MakeTransform` (`KismetMathLibrary.MakeVector` (.x (.location (`InstancedStaticMeshComponent.GetInstanceTransform` _hierarchicalinstancedstaticmesh _index false))) (.y (.location (`InstancedStaticMeshComponent.GetInstanceTransform` _hierarchicalinstancedstaticmesh _index false))) 2048.0) (.rotation (`InstancedStaticMeshComponent.GetInstanceTransform` _hierarchicalinstancedstaticmesh _index false)) (/ (.scale (`InstancedStaticMeshComponent.GetInstanceTransform` _hierarchicalinstancedstaticmesh _index false)) 50)) "AlwaysSpawn" "OverrideRootScale" null null))
  (bind _outactors (`GameplayStatics.GetAllActorsOfClass` "/Game/Blueprints/CharacterBlueprintSKMManny.CharacterBlueprintSKMManny_C"))
  (for (_array_element _array_index) _outactors
    (if (== _array_index 0)
      (bind _output_get (set `self.temporaryManny` _array_element))
      (bind _output_get_2 (set `/Game/Blueprints/CharacterBlueprintSKMManny.target` _output_get _output_get))
      (`self.SetActorTickEnabled` _output_get_2 false)
      (else
        (set `/Game/Blueprints/CharacterBlueprintSKMManny.target` (`self.temporaryManny`) _array_element)
        (set `self.temporaryManny` _array_element))))
  (bind _outactors_2 (`GameplayStatics.GetAllActorsOfClass` "/Game/Blueprints/CharacterBlueprintSKMMannySimple.CharacterBlueprintSKMMannySimple_C"))
  (for (_array_element_2 _array_index_2) _outactors_2
    (if (== _array_index_2 0)
      (bind _output_get_3 (set `self.temporaryMannySimple` _array_element_2))
      (bind _output_get_4 (set `/Game/Blueprints/CharacterBlueprintSKMMannySimple.target` _output_get_3 _output_get_3))
      (`self.SetActorTickEnabled` _output_get_4 false)
      (else
        (set `/Game/Blueprints/CharacterBlueprintSKMMannySimple.target` (`self.temporaryMannySimple`) _array_element_2)
        (set `self.temporaryMannySimple` _array_element_2))))
  (bind _outactors_3 (`GameplayStatics.GetAllActorsOfClass` "/Game/Blueprints/CharacterBlueprintSKMQuinn.CharacterBlueprintSKMQuinn_C"))
  (for (_array_element_3 _array_index_3) _outactors_3
    (if (== _array_index_3 0)
      (bind _output_get_5 (set `self.temporaryQuinn` _array_element_3))
      (bind _output_get_6 (set `/Game/Blueprints/CharacterBlueprintSKMQuinn.target` _output_get_5 _output_get_5))
      (`self.SetActorTickEnabled` _output_get_6 false)
      (else
        (set `/Game/Blueprints/CharacterBlueprintSKMQuinn.target` (`self.temporaryQuinn`) _array_element_3)
        (set `self.temporaryQuinn` _array_element_3))))
  (bind _outactors_4 (`GameplayStatics.GetAllActorsOfClass` "/Game/Blueprints/CharacterBlueprintSKMQuinnSimple.CharacterBlueprintSKMQuinnSimple_C"))
  (for (_array_element_4 _array_index_4) _outactors_4
    (if (== _array_index_4 0)
      (bind _output_get_7 (set `self.temporaryQuinnSimple` _array_element_4))
      (bind _output_get_8 (set `/Game/Blueprints/CharacterBlueprintSKMQuinnSimple.target` _output_get_7 _output_get_7))
      (`self.SetActorTickEnabled` _output_get_8 false)
      (else
        (set `/Game/Blueprints/CharacterBlueprintSKMQuinnSimple.target` (`self.temporaryQuinnSimple`) _array_element_4)
        (set `self.temporaryQuinnSimple` _array_element_4)))))

(fn `OnRep_HISMCArray`)

(fn `UserConstructionScript`)